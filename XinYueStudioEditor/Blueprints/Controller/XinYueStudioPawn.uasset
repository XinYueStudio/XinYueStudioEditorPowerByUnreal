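; Camera pawn for XinYueStudioEditor that gives mouse-driven rotate, pan and zoom with a visible cursor.
; On BeginPlay it possesses itself, stores its starting transform and arm length, and disables spring arm collision.
; Right-drag rotates the controller, the wheel changes arm length, and middle-drag pans along camera right/up, scaled by arm length.
; R restores the stored view; a leftover MouseX print shows arm length.
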(event `self.ReceiveBeginPlay`
  (bind _returnvalue (`GameplayStatics.GetPlayerController` 0))
  (bind _springarm (`self.SpringArm`))
  ;[1 1 1] Binding Pawn and Show Cursor
  (`Controller.Possess` _returnvalue self)
  (`WidgetBlueprintLibrary.SetInputMode_GameAndUIEx` _returnvalue null "DoNotLock" false)
  (set `PlayerController.bShowMouseCursor` true _returnvalue)
  ;[1 1 1] Read Original Position and Rotation
  (set `self.OlocalPosition` (`self.K2_GetActorLocation`))
  (set `self.OlocalRotation` (`Controller.GetControlRotation` (`GameplayStatics.GetPlayerController` 0)))
  (set `self.SpringArmLength` (`SpringArmComponent.TargetArmLength` _springarm))
  (set `SpringArmComponent.bDoCollisionTest` false _springarm))

(event `Key|RightMouseButton`
  (params (Key :type "Key Structure"))
  ;[1 1 1] Mouse Right Down Rotata Camera
  (:`Pressed`
    (set `self.RightMousePassed` true))
  (:`Released`
    (set `self.RightMousePassed` false)))

(event `InputAxisKey|MouseX`
  (params (AxisValue :type "Float (single-precision)"))
  (bind _returnvalue (`GameplayStatics.GetPlayerController` 0))
  (bind (_returnvalue_roll _returnvalue_pitch _returnvalue_yaw) (`KismetMathLibrary.BreakRotator` (`Controller.GetControlRotation` _returnvalue)))
  ;[1 1 1] Mouse Right Down Rotata Camera
  (if (`self.RightMousePassed`) :!label _label
    (`self.AddControllerYawInput` AxisValue)
    (`self.AddControllerPitchInput` (stale `InputAxis|InvertMouseY` AxisValue))
    (`Controller.SetControlRotation` _returnvalue (`KismetMathLibrary.MakeRotator` 0.0 _returnvalue_pitch _returnvalue_yaw))))

(event `InputAxis|InvertMouseY`
  (params (AxisValue :type "Float (single-precision)"))
  ;[1 1 1] Mouse Right Down Rotata Camera
  (goto _label))

(event `Key|MouseScrollUp`
  (params (Key :type "Key Structure"))
  (bind _springarm (`self.SpringArm`))
  ;[1 1 1] Mouse Wheel Scale
  (:`Pressed`
    (set `SpringArmComponent.TargetArmLength` (- (`SpringArmComponent.TargetArmLength` _springarm) 20.0) _springarm)))

(event `Key|MouseScrollDown`
  (params (Key :type "Key Structure"))
  (bind _springarm (`self.SpringArm`))
  ;[1 1 1] Mouse Wheel Scale
  (:`Pressed`
    (set `SpringArmComponent.TargetArmLength` (- (`SpringArmComponent.TargetArmLength` _springarm) -20.0) _springarm)))

(event `Key|MiddleMouseButton`
  (params (Key :type "Key Structure"))
  ;[1 1 1] Middle Mouse Move
  (:`Pressed`
    (set `self.MiddleMousePassed` true))
  (:`Released`
    (set `self.MiddleMousePassed` false)))

(event `self.ReceiveTick`
  (params (DeltaSeconds :type "Float (single-precision)"))
  (bind _returnvalue (`SceneComponent.K2_GetComponentRotation` (`self.Camera`)))
  (bind _returnvalue_2 (`KismetMathLibrary.Abs` (`SpringArmComponent.TargetArmLength` (`self.SpringArm`))))
  ;[1 1 1] Middle Mouse Move
  (if (`self.MiddleMousePassed`)
    (`self.AddMovementInput` (`KismetMathLibrary.GetRightVector` _returnvalue) (* (* (stale `InputAxisKey|MouseX` AxisValue) -1.0) _returnvalue_2))
    (`self.AddMovementInput` (`KismetMathLibrary.GetUpVector` _returnvalue) (* (* (stale `InputAxisKey|MouseY` AxisValue) -1.0) _returnvalue_2))))

(event `InputAxisKey|MouseX`
  (params (AxisValue :type "Float (single-precision)"))
  (bind _targetarmlength (`SpringArmComponent.TargetArmLength` (`self.SpringArm`)))
  ;[1 1 1] Middle Mouse Move
  (`KismetSystemLibrary.PrintString` (`KismetStringLibrary.Conv_DoubleToString` _targetarmlength) true true (struct :`G` 0.66 :`B` 1.0 :`A` 1.0) _targetarmlength))

(event `InputAxisKey|MouseY`
  (params (AxisValue :type "Float (single-precision)"))
  ;[1 1 1] Middle Mouse Move
)

(event `Key|R`
  (params (Key :type "Key Structure"))
  ;[1 1 1] Reset All Data
  (:`Pressed`
    (`self.K2_SetActorLocation` (`self.OlocalPosition`))
    (`Controller.SetControlRotation` (`GameplayStatics.GetPlayerController` 0) (`self.OlocalRotation`))
    (set `SpringArmComponent.TargetArmLength` (`self.SpringArmLength`) (`self.SpringArm`))))

(fn `UserConstructionScript`)